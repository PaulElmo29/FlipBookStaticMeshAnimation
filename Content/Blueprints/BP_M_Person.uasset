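; BP_M_Person is an AI-driven walking person that animates as a mesh flipbook and wanders at random.
; Each Tick swaps the InstancedStaticMesh component to the next mesh in a looping array, instead of using skeletal animation.
; Tick also resets its own interval to DeltaSeconds multiplied by TickInterval.
; From BeginPlay, RandomWalks moves it slowly to random reachable nearby points, repeating only when a move succeeds.
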(event `self.ReceiveTick`
  (params (DeltaSeconds :type "Float (single-precision)"))
  ;[0 0 0 1 22] FlipBook Animation using the static mesh
  (`self.SetActorTickInterval` (* DeltaSeconds (`self.TickInterval`)))
  (bind _output_get (set `self.AnimationIndex` (+ (`self.AnimationIndex`) 1)))
  (if (> _output_get (`self.AnimationFrameCounts`))
    (set `self.AnimationIndex` 0))
  (`StaticMeshComponent.SetStaticMesh` (`self.InstancedStaticMesh`) (`|GetArrayItem` (`self.AnimationStaticMeshes`) (`self.AnimationIndex`))))

(event `self.ReceiveBeginPlay`
  (`self.RandomWalks`))

(event `RandomWalks`
  ;[0 1 0.04508] AI
  (set `CharacterMovementComponent.MaxWalkSpeed` 100.0 (`self.CharacterMovement`))
  (`|AIMoveTo` self (`NavigationSystemV1.K2_GetRandomReachablePointInRadius` (`self.K2_GetActorLocation`) 1000.0 null null) null
    (:`OnSuccess`
      (`self.RandomWalks`))))

(fn `UserConstructionScript`)